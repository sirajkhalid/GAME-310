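; BP_PauseManager is an actor that toggles the pause menu from the IA_Pause input action, enabling input from player controller 0 on BeginPlay.
; With no menu open, it creates and stores a PauseMenu widget, switches to game-and-UI input, shows the cursor and pauses the game.
; With a menu open, it removes the widget and restores game-only input.
; The nodes that hide the cursor and unpause are disconnected and never run.
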(event Input|EnhancedActionEvents|EnhancedInputActionIA_Pause
  (params (ActionValue :type Boolean) (ElapsedSeconds :type Float%20%28double-precision%29) (TriggeredSeconds :type Float%20%28double-precision%29) (InputAction :type Input%20Action%20Object%20Reference :default "/Game/Input/IA_Pause.IA_Pause"))
  (bind _returnvalue (Game|GetPlayerController 0))
  (Utilities|IsValid (Variables|Components|GetPauseUIRef)
    (:Is%20Valid
      (Widget|RemovefromParent (Variables|Components|GetPauseUIRef))
      (Variables|Components|SetPauseUIRef 0)
      (Input|SetInputModeGameOnly (Game|GetPlayerController 0) false))
    (:Is%20Not%20Valid
      (bind _returnvalue_2 (UserInterface|CreateWidget "/Game/UI/PauseMenu.PauseMenu_C"))
      (bind _output_get (Variables|Components|SetPauseUIRef _returnvalue_2))
      (UserInterface|Viewport|AddtoViewport _output_get 0)
      (Input|SetInputModeGameandUI _returnvalue 0 "DoNotLock" true false)
      (Variables|/Script/Engine.PlayerController|SetbShowMouseCursor _returnvalue true)
      (Game|SetGamePaused true))))

(event EventBeginPlay
  (Input|EnableInput (Game|GetPlayerController 0)))

(event Collision|EventActorBeginOverlap
  (params (OtherActor :type Actor%20Object%20Reference)))

(event EventTick
  (params (DeltaSeconds :type Float%20%28single-precision%29)))

(fn ConstructionScript)